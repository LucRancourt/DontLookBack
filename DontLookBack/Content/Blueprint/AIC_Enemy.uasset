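; AIC_Enemy is an enemy AI controller that detects whether the player is looking toward its pawn.
; One second after possession it runs BT_Enemy, stores the first-person character as the Blackboard target and opens a gate for Tick.
; Each tick, a dot product between camera forward and the direction to the pawn sets the player-looking key.
; Audio plays while the player looks and stops otherwise.
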(event `self.ReceivePossess`
  (params (PossessedPawn :type "Pawn Object Reference"))
  (bind _playerlookingkeyname (`self.PlayerLookingKeyName`))
  (bind _blackboard (`self.Blackboard`))
  (bind _playercamref (`self.PlayerCamRef`))
  (bind _audio (`self.Audio`))
  (`KismetSystemLibrary.Delay` 1.0)
  (`self.RunBehaviorTree` "/Game/Blueprint/BT_Enemy.BT_Enemy")
  (bind _returnvalue (`GameplayStatics.GetActorOfClass` "/Game/FirstPerson/Blueprints/BP_FirstPersonCharacter.BP_FirstPersonCharacter_C"))
  (`BlackboardComponent.SetValueAsObject` _blackboard (`self.TargetKeyName`) _returnvalue)
  (set `self.PlayerCamRef` (`/Game/FirstPerson/Blueprints/BP_FirstPersonCharacter.FirstPersonCamera` _returnvalue))
  (goto _label :!via `Open`))

(event `self.ReceiveTick`
  (params (DeltaSeconds :type "Float (single-precision)"))
  (bind _playerlookingkeyname (`self.PlayerLookingKeyName`))
  (bind _blackboard (`self.Blackboard`))
  (bind _playercamref (`self.PlayerCamRef`))
  (bind _audio (`self.Audio`))
  (`/Engine/EditorBlueprintResources/StandardMacros.Gate` true :!label _label
    (:`Exit`
      (if (`KismetMathLibrary.InRange_FloatFloat` (`KismetMathLibrary.Dot_VectorVector` (`KismetMathLibrary.Normal` (- (`self.K2_GetActorLocation` (`self.K2_GetPawn`)) (`SceneComponent.K2_GetComponentLocation` _playercamref))) (`SceneComponent.GetForwardVector` _playercamref)) 0.8)
        (`BlackboardComponent.SetValueAsBool` _blackboard _playerlookingkeyname true)
        (if (not (`AudioComponent.IsPlaying` _audio))
          (`AudioComponent.Play` _audio 0.0))
        (else
          (`BlackboardComponent.SetValueAsBool` _blackboard _playerlookingkeyname false)
          (`AudioComponent.Stop` _audio))))))

(fn `UserConstructionScript`)