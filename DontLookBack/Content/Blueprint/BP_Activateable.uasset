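; BP_Activateable is an interactable actor tinted by its NeededColor, with a placeholder activation response.
; The construction script creates a dynamic M_Color material on its mesh and sets BaseColor from that color enum.
; Interact and DoStuff only print debug messages, while Highlight and EndInteract are empty.
; The activator and highlight color getters return fixed values, and nothing here compares NeededColor against an activator.
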(event `/Game/Interfaces/BPI_Interactable.Highlight`
  (params (`Turn ON` :type Boolean)))

(event `/Game/Interfaces/BPI_Interactable.EndInteract`)

(event `/Game/Interfaces/BPI_Interactable.Interact`
  (params (Caller :type "Actor Object Reference"))
  (`KismetSystemLibrary.PrintString` "Hello"))

(fn `DoStuff`
  (`KismetSystemLibrary.PrintString` "You Win!"))

(fn `GetActivatorColor`
  (returns (ActivatorColor :type "/Game/Enum/E_Colors Enum"))
  (return "NewEnumerator0"))

(fn `GetHighlightColor`
  (returns (Color :type "LinearColor Structure"))
  (return))

(fn `UserConstructionScript`
  (bind _returnvalue (`PrimitiveComponent.CreateDynamicMaterialInstance` (`self.StaticMesh`) 0 "/Game/Materials/M_Color.M_Color" "None"))
  (bind _color (`/Game/Blueprint/BPFL_GeneralStuff.GetColorFromEColor` (`self.NeededColor`)))
  (`MaterialInstanceDynamic.SetVectorParameterValue` _returnvalue "BaseColor" _color))